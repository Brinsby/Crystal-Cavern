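; BP_Cannon is an automatic cannon actor that repeatedly fires BP_Projectile from the moment play begins.
; Each cycle waits for the fire-rate delay, then spawns a scaled projectile at the Arrow component's world location and rotation.
; A recoil timeline then slides the barrel along its relative Y axis, and its Cannon Fired event track restarts the delay, closing the loop without a timer.
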(event EventBeginPlay
  (Utilities|FlowControl|Delay (Variables|CanonProperties|GetCanonFireRate) :!label _label)
  (CallFunction|SpawnProjectile)
  (bind _canonrecoil (Timeline|RecoilTimeline PlayFromStart)
    (:Update
      (CallFunction|MoveCannonBarrel _canonrecoil))
    (:CannonFired
      (goto _label))))

(fn ConstructionScript)

(fn SpawnProjectile
  (bind _arrow (Variables|Default|GetArrow))
  (Game|SpawnActorfromClass "/Game/Blueprints/Actors/Projectiles/BP_Projectile.BP_Projectile_C" (Math|Transform|MakeTransform (Transformation|GetWorldLocation _arrow) (Transformation|GetWorldRotation _arrow) (Math|Conversions|ToVector(Float) (Variables|CanonProperties|GetProjectileScale))) "Undefined" 0 0))

(fn MoveCannonBarrel
  (params (CannonBarrelYLocation :type Float%20%28single-precision%29))
  (Transformation|SetRelativeLocation (Variables|Default|GetBarrel) (Math|Vector|MakeVector 0.0 CannonBarrelYLocation 0.0) false false))