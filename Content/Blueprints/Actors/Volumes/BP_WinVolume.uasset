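; Win volume actor that ends or advances the game when the player overlaps it.
; If any BP_Crystal actors remain in the world, it quits the game, despite the check's name CheckIfAllCrystalsCollected.
; Otherwise, it finds the current level in the LevelNames array and opens the next entry by name.
; On the final listed level, completion does nothing.
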(event Collision|EventActorBeginOverlap
  (params (OtherActor :type Actor%20Object%20Reference))
  (Utilities|IsPlayer OtherActor
    (:IsPlayer
      (if (CallFunction|CheckifAllCrystalsCollected)
        (Game|QuitGame 0 "Quit" false)
        (else
          (LevelManagement|CompleteLevel))))))

(fn ConstructionScript)

(fn CheckifAllCrystalsCollected
  (bind _outactors (Actor|GetAllActorsOfClass "/Game/Blueprints/Actors/Collectables/BP_Crystal.BP_Crystal_C"))
  (return (> (Utilities|Array|Length _outactors) 0)))

(fn CompleteLevel
  (if (not (LevelManagement|IsFinalLevel))
    (LevelManagement|LoadNextLevel)))

(fn GetCurrentLevelIndex
  (bind _returnvalue (Game|GetCurrentLevelName true))
  (return (Utilities|Array|FindItem (Variables|Default|GetLevelNames) (Utilities|String|StringToName _returnvalue))))

(fn IsFinalLevel
  (return (== (LevelManagement|GetCurrentLevelIndex) (Utilities|Array|LastIndex (Variables|Default|GetLevelNames)))))

(fn LoadNextLevel
  (Game|OpenLevel(byName) (LevelManagement|GetNextLevelName)))

(fn GetNextLevelName
  (return (Utilities|Array|Get(acopy) (Variables|Default|GetLevelNames) (+ (LevelManagement|GetCurrentLevelIndex) 1))))