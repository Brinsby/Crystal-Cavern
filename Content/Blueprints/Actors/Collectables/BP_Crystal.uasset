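; BP_Crystal is a collectable crystal that plays a pickup animation when the player overlaps it, then destroys itself.
; On overlap it stores its scale and point light intensity, then plays CollectionTimeline.
; Timeline curves drive it toward the player, shrink it to zero and modulate the light relative to its starting intensity.
; Movement lerps from the top half's current location to the player's live position, so it homes in cumulatively.
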(event Collision|EventActorBeginOverlap
  (params (OtherActor :type Actor%20Object%20Reference))
  (Utilities|IsPlayer OtherActor
    (:IsPlayer
      (CallFunction|SetStartingLightIntensity)
      (CallFunction|StoreActorScale)
      (bind (_direction _collectionprogress _scaleprogress _lightintensity) (Timeline|CollectionTimeline Play)
        (:Update
          (CallFunction|MovetoPlayer (Game|Player|GetPlayerPawn 0) _collectionprogress)
          (CallFunction|ScaleCrystal _scaleprogress)
          (CallFunction|AdjustLight _lightintensity))
        (:Finished
          (Actor|DestroyActor))))))

(fn ConstructionScript)

(fn MovetoPlayer
  (params (self2 :type Actor%20Object%20Reference) (Alpha :type Float%20%28single-precision%29))
  (Transformation|SetActorLocation (Math|Vector|Lerp(Vector) (Transformation|GetWorldLocation (Variables|Default|GetCrystalTopHalf)) (Transformation|GetActorLocation self2) Alpha) false false))

(fn StoreActorScale
  (Variables|Default|SetStartScale (Transformation|GetActorScale3D)))

(fn ScaleCrystal
  (params (Alpha :type Float%20%28single-precision%29))
  (Transformation|SetActorScale3D (Math|Vector|Lerp(Vector) (Variables|Default|GetStartScale) "0, 0, 0" Alpha)))

(fn AdjustLight
  (params (LightIntensityValue :type Float%20%28single-precision%29))
  (Rendering|Components|Light|SetIntensity (Variables|Default|GetPointLight) (Math|Float|Lerp 0.0 (Variables|Default|GetStartLightIntensity) LightIntensityValue)))

(fn SetStartingLightIntensity
  (Variables|Default|SetStartLightIntensity (Variables|/Script/Engine.LightComponentBase|GetIntensity (Variables|Default|GetPointLight))))